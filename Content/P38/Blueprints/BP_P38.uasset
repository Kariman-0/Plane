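; BP_P38 is a P38 actor that flies itself along its local X axis at a constant slow speed while spinning its parts.
; Each Tick rolls the Left and Right components at the same fast rate, likely as the twin propellers, and offsets the whole actor forward.
; Both motions scale by delta time to stay frame-rate independent, with no input, physics or construction logic.
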(event EventTick
  (params (DeltaSeconds :type Float%20%28single-precision%29))
  (Variables|Default|SetSpeed01 (* DeltaSeconds 5.4e+03))
  (Transformation|AddLocalRotation (Variables|Default|GetLeft) (Math|Rotator|MakeRotator (Variables|Default|GetSpeed01) 0.0 0.0) false false)
  (Transformation|AddLocalRotation (Variables|Default|GetRight) (Math|Rotator|MakeRotator (Variables|Default|GetSpeed01) 0.0 0.0) false false)
  (Transformation|AddActorLocalOffset (Math|Vector|MakeVector (* (Utilities|Time|GetWorldDeltaSeconds) 2e+01) 0.0 0.0) false false))

(fn ConstructionScript)